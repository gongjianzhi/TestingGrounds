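; BP_Tile is one segment of the infinite terrain, filled on BeginPlay with enemy characters and props.
; Enemy count range scales with the game mode's Score, while props use per-type spawn caps and radii.
; The Barrier starts per IsLock and locks red when the player enters LockingVolume.
; On player exit, the tile asks the game mode for the next tile, reports itself conquered and destroys itself.
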(event `self.ReceiveBeginPlay`
  (if (`self.IsLock`)
    (`self.Lock`)
    (else
      (`self.Unlock`)))
  (bind _asbp_infinite_terrain_game_mode (cast `/Game/Dynamic/BP_InfiniteTerrainGameMode` (`GameplayStatics.GetGameMode`)))
  (bind _score (`/Game/Dynamic/BP_InfiniteTerrainGameMode.Score` _asbp_infinite_terrain_game_mode))
  (`self.PlaceAIPawns` "/Game/Dynamic/Character/Behavior/BP_Character.BP_Character_C" (+ _score (`self.MinEnemyNum`)) (+ _score (`self.MaxEnemyNum`)) 100.0)
  (`self.PlaceActors` "/Game/Dynamic/Terrain/Props/BP_Barrel_1.BP_Barrel_1_C" 0 3 100.0)
  (`self.PlaceActors` "/Game/Dynamic/Terrain/Props/BP_Barrel_2.BP_Barrel_2_C" 0 3 100.0)
  (`self.PlaceActors` "/Game/Dynamic/Terrain/Props/BP_Barrel_3.BP_Barrel_3_C" 0 3 30.0)
  (`self.PlaceActors` "/Game/Dynamic/Terrain/Props/BP_Barrel_4.BP_Barrel_4_C" 0 3 30.0)
  (`self.PlaceActors` "/Game/Dynamic/Terrain/Props/BP_Box_1.BP_Box_1_C" 0 4 80.0)
  (`self.PlaceActors` "/Game/Dynamic/Terrain/Props/BP_Box_2.BP_Box_2_C" 0 4 150.0)
  (`self.PlaceActors` "/Game/Dynamic/Terrain/Props/BP_Box_3.BP_Box_3_C" 0 4 150.0)
  (`self.PlaceActors` "/Game/Dynamic/Terrain/Props/BP_Box_4.BP_Box_4_C" 0 4 120.0)
  (`self.PlaceActors` "/Game/Dynamic/Terrain/Props/BP_Rack_1.BP_Rack_1_C" 0 5 200.0)
  (`self.PlaceActors` "/Game/Dynamic/Terrain/Props/BP_Rack_2.BP_Rack_2_C" 0 5 200.0)
  (`self.PlaceActors` "/Game/Dynamic/Terrain/Props/BP_Rack_3.BP_Rack_3_C" 0 5 280.0)
  (`self.PlaceActors` "/Game/Dynamic/Terrain/Props/BP_Rack_4.BP_Rack_4_C" 0 5 300.0)
  (`self.PlaceActors` "/Game/Dynamic/Terrain/Props/BP_Rack_5.BP_Rack_5_C" 0 5 300.0)
  (`self.PlaceActors` "/Game/Dynamic/Terrain/Props/BP_Tarp_1.BP_Tarp_1_C" 0 2 150.0)
  (`self.PlaceActors` "/Game/Dynamic/Terrain/Props/BP_Tarp_2.BP_Tarp_2_C" 0 2 50.0)
  (`self.PlaceActors` "/Game/Dynamic/Terrain/Props/BP_Tarp_3.BP_Tarp_3_C" 0 2 30.0)
  (`self.PlaceActors` "/Game/Dynamic/Terrain/Props/BP_TrafficBarrel.BP_TrafficBarrel_C" 0 2 50.0)
  (`self.PlaceActors` "/Game/Dynamic/Terrain/Props/BP_WaterTank.BP_WaterTank_C" 0 2 90.0))

(event `self.LockingVolume.OnComponentBeginOverlap`
  (params (OverlappedComponent :type "PrimitiveComponent Object Reference") (OtherActor :type "Actor Object Reference") (OtherComp :type "PrimitiveComponent Object Reference") (OtherBodyIndex :type Integer) (bFromSweep :type Boolean) (SweepResult :type "HitResult Structure (by ref)"))
  (`self.IsPlayerActor` OtherActor)
  (`self.Lock`))

(event `self.LockingVolume.OnComponentEndOverlap`
  (params (OverlappedComponent :type "PrimitiveComponent Object Reference") (OtherActor :type "Actor Object Reference") (OtherComp :type "PrimitiveComponent Object Reference") (OtherBodyIndex :type Integer))
  (`self.IsPlayerActor` OtherActor)
  (if (not (`self.IsSpawnedNextTile`))
    (bind _asbp_infinite_terrain_game_mode (cast `/Game/Dynamic/BP_InfiniteTerrainGameMode` (`GameplayStatics.GetGameMode`)))
    (`/Game/Dynamic/BP_InfiniteTerrainGameMode.SpawnNextTile` _asbp_infinite_terrain_game_mode)
    (`self.TileConquered`)
    (set `self.IsSpawnedNextTile` true)
    (`self.K2_DestroyActor`)))

(fn `Get Attach Location`
  (returns (`Attach Transform` :type "Transform Structure"))
  (return (`SceneComponent.K2_GetComponentToWorld` (`self.Arrow`))))

(fn `Lock`
  (`PrimitiveComponent.SetCollisionEnabled` (`self.Barrier`) "QueryAndPhysics")
  (`PrimitiveComponent.SetMaterial` (`self.Barrier`) 0 "/Game/Dynamic/Terrain/MI_Barrier_Red.MI_Barrier_Red"))

(fn `TileConquered`
  (if (not (`self.IsSpawnedNextTile`))
    (bind _asbp_infinite_terrain_game_mode (cast `/Game/Dynamic/BP_InfiniteTerrainGameMode` (`GameplayStatics.GetGameMode`)))
    (`/Game/Dynamic/BP_InfiniteTerrainGameMode.NewTileConquered` _asbp_infinite_terrain_game_mode)
    (set `self.IsSpawnedNextTile` true)))

(fn `Unlock`
  (`PrimitiveComponent.SetCollisionEnabled` (`self.Barrier`) "NoCollision")
  (`PrimitiveComponent.SetMaterial` (`self.Barrier`) 0 "/Game/Dynamic/Terrain/MI_Barrier_Green.MI_Barrier_Green"))

(fn `UserConstructionScript`)